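; An interactive lamp actor that moves its top piece and toggles its light when overlapped.
; On BeginPlay it spawns separate bottom and top actors at vertical offsets from itself.
; Overlap begin plays a timeline offsetting the top from its captured location, and overlap end reverses it.
; When the timeline finishes, it either spawns a light actor above that location or destroys the existing one.
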(event EventBeginPlay
  (bind _returnvalue (Transformation|GetActorLocation))
  (bind _returnvalue_2 (Transformation|GetActorRotation))
  (bind _returnvalue_3 (Math|Vector|MakeVector 1.0 1.0 1.0))
  (Variables|Default|SetinitialLampTransform (Transformation|GetActorTransform))
  (bind _returnvalue_4 (Game|SpawnActorfromClass "/Game/BP_LAMPBOT.BP_LAMPBOT_C" (Math|Transform|MakeTransform (+ (Math|Vector|MakeVector 0.0 0.0 35.0) _returnvalue) _returnvalue_2 _returnvalue_3) "Undefined" 0 0))
  (Variables|Default|SetBOT _returnvalue_4)
  (bind _returnvalue_5 (Game|SpawnActorfromClass "/Game/BP_LAMPTOP.BP_LAMPTOP_C" (Math|Transform|MakeTransform (+ _returnvalue (Math|Vector|MakeVector 0.0 0.0 105.0)) _returnvalue_2 _returnvalue_3) "Undefined" 0 0))
  (Variables|Default|SetTOP _returnvalue_5))

(event Collision|EventActorBeginOverlap
  (params (OtherActor :type Actor%20Object%20Reference))
  (Variables|Default|SetTopLoc (Transformation|GetActorLocation (Variables|Default|GetTOP)))
  (bind _top (Timeline|Timeline_0 Play)
    (:Update
      (Transformation|SetActorLocation (Variables|Default|GetTOP) (+ (Variables|Default|GetTopLoc) _top) false false))
    (:Finished
      (if (Variables|Default|GetLightOn)
        (Actor|DestroyActor (Variables|Default|GetLight))
        (Variables|Default|SetLightOn false)
        (else
          (bind _returnvalue (Game|SpawnActorfromClass "/Game/BP_LampLight.BP_LampLight_C" (Math|Transform|MakeTransform (- (Variables|Default|GetTopLoc) (Math|Vector|MakeVector 0.0 0.0 -125.0)) (Transformation|GetActorRotation) (Transformation|GetActorScale3D)) "Undefined" 0 0))
          (Variables|Default|SetLight _returnvalue)
          (Variables|Default|SetLightOn true))))))

(event Collision|EventActorEndOverlap
  (params (OtherActor :type Actor%20Object%20Reference))
  (bind _top (Timeline|Timeline_0 Reverse)
    (:Update
      (Transformation|SetActorLocation (Variables|Default|GetTOP) (+ (Variables|Default|GetTopLoc) _top) false false))
    (:Finished
      (if (Variables|Default|GetLightOn)
        (Actor|DestroyActor (Variables|Default|GetLight))
        (Variables|Default|SetLightOn false)
        (else
          (bind _returnvalue (Game|SpawnActorfromClass "/Game/BP_LampLight.BP_LampLight_C" (Math|Transform|MakeTransform (- (Variables|Default|GetTopLoc) (Math|Vector|MakeVector 0.0 0.0 -125.0)) (Transformation|GetActorRotation) (Transformation|GetActorScale3D)) "Undefined" 0 0))
          (Variables|Default|SetLight _returnvalue)
          (Variables|Default|SetLightOn true))))))

(fn ConstructionScript)