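; BP_TriggerGate is a trigger actor that moves two referenced block actors when any actor overlaps it.
; The overlap caches both block locations, then plays a timeline that adds offsets to them without sweep.
; The track names are crossed: the BlockTwo track drives BlockOne and the BlockOne track drives BlockTwo.
; The trigger destroys itself when the timeline finishes, with no guard against repeat overlaps during playback.
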(event Collision|EventActorBeginOverlap
  (params (OtherActor :type Actor%20Object%20Reference))
  (Variables|Default|SetBlockOneLoc (Transformation|GetActorLocation (Variables|Default|GetBlockOne)))
  (Variables|Default|SetBlockTwoLoc (Transformation|GetActorLocation (Variables|Default|GetBlockTwo)))
  (bind (_direction _blockone _blocktwo) (Timeline|Timeline_0 Play)
    (:Update
      (Transformation|SetActorLocation (Variables|Default|GetBlockOne) (+ (Variables|Default|GetBlockOneLoc) _blocktwo) false false)
      (Transformation|SetActorLocation (Variables|Default|GetBlockTwo) (+ (Variables|Default|GetBlockTwoLoc) _blockone) false false))
    (:Finished
      (Actor|DestroyActor))))

(fn ConstructionScript)