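; BP_Bullet is a battle-system projectile that flies in a straight line and destroys itself when it hits the player.
; Tick moves it along world X with sweep, by Speed divided by DeltaSeconds, so travel depends on frame rate.
; Hit destroys it only for an exact BP_PlayerCharacter class match and applies no damage.
; Look-at aiming toward the player exists only as disconnected nodes that never run.
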(event EventBeginPlay)

(event Collision|EventActorBeginOverlap
  (params (OtherActor :type Actor%20Object%20Reference)))

(event EventTick
  (params (DeltaSeconds :type Float%20%28single-precision%29))
  (Class|Actor|AddActorWorldTransform (Math|Transform|MakeTransform (Math|Vector|MakeVector (/ (Variables|Default|Getspeed) DeltaSeconds) 0.0 0.0)) true false))

(event Collision|EventHit
  (params (MyComp :type Primitive%20Component%20Object%20Reference) (Other :type Actor%20Object%20Reference) (OtherComp :type Primitive%20Component%20Object%20Reference) (bSelfMoved :type Boolean) (HitLocation :type Vector :default "0, 0, 0") (HitNormal :type Vector :default "0, 0, 0") (NormalImpulse :type Vector :default "0, 0, 0") (Hit :type Hit%20Result%20Structure%20%28by%20ref%29))
  (if (== (Utilities|GetClass Other) "/Game/ThirdPersonBP/Blueprints/BP_PlayerCharacter.BP_PlayerCharacter_C")
    (Actor|DestroyActor)))

(fn ConstructionScript)