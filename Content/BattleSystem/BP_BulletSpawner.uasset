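; Battle-system spawner actor that fires timed waves of BP_Bullet_IDK projectiles downward from offsets around its own location.
; WaveSpawnTrigger starts a Delay, DoN and Gate loop that fires a limited run of waves, and StopBullets closes the gate to halt it.
; Each wave randomly picks Flat Wave (parallel) or X Pattern (crossing), with SpawnBullet aiming each of four bullets by look-at rotation.
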(event Custom|WaveSpawnTrigger
  (Utilities|FlowControl|Sequence
    (:then_0
      (goto _label_3 Open))
    (:then_1
      (Utilities|FlowControl|Sequence
        (:then_0
          (CallFunction|SpawnWave (Utilities|Enum|ByteToEnumPatterns (Math|Conversions|ToByte(Integer) (Math|Random|RandomIntegerinRange 0 1))) :!label _label)
          (Utilities|FlowControl|Delay 2.0)
          (Utilities|FlowControl|DoN 5 :!label _label_2
            (:Exit
              (Utilities|FlowControl|Gate true :!label _label_3
                (:Exit
                  (goto _label))))))
        (:then_1
          (goto _label_2 Reset))))))

(event Custom|Stop%20Bullets
  (Utilities|FlowControl|Gate true) ; enters at Close
)

(event EventBeginPlay)

(event Collision|EventActorBeginOverlap
  (params (OtherActor :type Actor%20Object%20Reference)))

(fn ConstructionScript)

(fn SpawnBullet
  (params (Target%20Loc :type Vector) (Start%20Loc :type Vector))
  (Game|SpawnActorfromClass "/Game/Runner_Content/Blueprints/BP_Bullet_IDK.BP_Bullet_IDK_C" (Math|Transform|MakeTransform Start%20Loc (Math|Rotator|FindLookatRotation Start%20Loc Target%20Loc)) "Undefined" 0 0))

(fn SpawnWave
  (params (Pattern :type Patterns%20Enum))
  (bind _returnvalue (Transformation|GetActorLocation))
  (bind _returnvalue_2 (Transformation|GetActorLocation))
  (switch Utilities|FlowControl|Switch|SwitchonPatterns Pattern
    (:NewEnumerator0
      (Utilities|FlowControl|Sequence
        (:then_0
          (CallFunction|SpawnBullet (+ _returnvalue_2 "200.000000,0.000000,-1000.000000") (+ _returnvalue_2 "200.000000,0.000000, 0")))
        (:then_1
          (CallFunction|SpawnBullet (+ _returnvalue_2 "500.000000,0.000000,-1000.000000") (+ _returnvalue_2 "500.000000,0.000000, 0")))
        (:then_2
          (CallFunction|SpawnBullet (+ _returnvalue_2 "-200.000000,0.000000,-1000.000000") (+ _returnvalue_2 "-200.000000,0.000000, 0")))
        (:then_3
          (CallFunction|SpawnBullet (+ _returnvalue_2 "-500.000000,0.000000,-1000.000000") (+ _returnvalue_2 "-500.000000,0.000000, 0")))))
    (:NewEnumerator1
      (Utilities|FlowControl|Sequence
        (:then_0
          (CallFunction|SpawnBullet (+ _returnvalue "800.000000,0.000000,-1000.000000") (+ _returnvalue "-800.000000,0.000000, 0")))
        (:then_1
          (CallFunction|SpawnBullet (+ _returnvalue "500.000000,0.000000,-1000.000000") (+ _returnvalue "-500.000000,0.000000, 0")))
        (:then_2
          (CallFunction|SpawnBullet (+ _returnvalue "-800.000000,0.000000,-1000.000000") (+ _returnvalue "800.000000,0.000000, 0")))
        (:then_3
          (CallFunction|SpawnBullet (+ _returnvalue "-500.000000,0.000000,-1000.000000") (+ _returnvalue "500.000000,0.000000, 0")))))))