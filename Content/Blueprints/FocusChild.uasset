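; FocusChild is a clickable mesh actor that the player picks as the ThirdPersonCharacter's focus target.
; Construction caches original materials, creates a dynamic selection material and seeds health from MaxHealth.
; Clicking registers it as FocusTarget, disables input on the first FocusParent and re-enables the character's input.
; Tick polls to show selection or original materials, switching to a destroyed material and locking it once health reaches zero.
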(event OnEndCursorOver(StaticMesh)
  (params (TouchedComponent :type Primitive%20Component%20Object%20Reference))
  ;[1 1 1] Change Mesh Materials
  (if (not (Variables|Default|GetisSelectedObject))
    (if (not (Variables|Default|GetobjDeleted))
      (for _index (range 0 (Utilities|Array|Length (Rendering|Material|GetMaterials (Variables|Default|GetStaticMesh))))
        (Rendering|Material|SetMaterial (Variables|Default|GetStaticMesh) _index (Utilities|Array|Get(acopy) (Variables|Default|GetoriginalMaterials) _index))))))

(event Custom|objectDestroyed
  (for _index (range 0 (Utilities|Array|Length (Rendering|Material|GetMaterials (Variables|Default|GetStaticMesh))))
    (Rendering|Material|SetMaterial (Variables|Default|GetStaticMesh) _index "/Game/Blueprints/FocusObject_Destroyed.FocusObject_Destroyed")
    (Variables|Default|SetobjDeleted true)))

(event EventBeginPlay)

(event Collision|EventActorBeginOverlap
  (params (OtherActor :type Actor%20Object%20Reference)))

(event EventTick
  (params (DeltaSeconds :type Float%20%28single-precision%29))
  (bind _staticmesh (Variables|Default|GetStaticMesh))
  (bind _staticmesh_2 (Variables|Default|GetStaticMesh))
  (bind _returnvalue (Rendering|Material|GetMaterials _staticmesh_2))
  (bind _returnvalue_2 (Utilities|Array|Length _returnvalue))
  ;[1 1 1] Change Mesh Materials
  (if (<= (Variables|Default|GetchildHealth) 0.0)
    (Variables|Default|SetobjDeleted true)
    (CallFunction|ObjectDestroyed)
    (else
      (bind _asthird_person_character (Utilities|Casting|CastToThirdPersonCharacter (Game|GetPlayerCharacter 0)))
      (if (== (Variables|/Game/ThirdPersonBP/Blueprints/ThirdPersonCharacter.ThirdPersonCharacter_C|GetfocusTarget _asthird_person_character) self)
        (if (not (Variables|Default|GetobjDeleted))
          (for _index (range 0 _returnvalue_2)
            (Rendering|Material|SetMaterial _staticmesh _index (Variables|Default|GetselectionMat))))
        (elif (not (Variables|Default|GetobjDeleted))
          (for _index_2 (range 0 _returnvalue_2)
            (Rendering|Material|SetMaterial _staticmesh _index_2 (Utilities|Array|Get(acopy) (Variables|Default|GetoriginalMaterials) _index_2))))))))

(event MouseInput|EventActorOnClicked
  (params (ButtonPressed :type Key%20Structure :default "AnyKey"))
  (bind _returnvalue (Game|GetPlayerController 0))
  ;[1 1 1] Handle selection of focus target
  (if (not (Variables|Default|GetobjDeleted))
    (if (Variables|Default|GetcanSelect)
      _
      (else
        _))
    (bind _asthird_person_character (Utilities|Casting|CastToThirdPersonCharacter (Game|GetPlayerCharacter 0)))
    (Variables|/Game/ThirdPersonBP/Blueprints/ThirdPersonCharacter.ThirdPersonCharacter_C|SetcanSelectFocusObject _asthird_person_character false)
    (bind _output_get (Variables|/Game/ThirdPersonBP/Blueprints/ThirdPersonCharacter.ThirdPersonCharacter_C|SetfocusObjectChosen _asthird_person_character true))
    (bind _output_get_2 (Variables|/Game/ThirdPersonBP/Blueprints/ThirdPersonCharacter.ThirdPersonCharacter_C|SetfocusTarget _asthird_person_character self))
    (for _index (range 0 (Utilities|Array|Length (Rendering|Material|GetMaterials (Variables|FocusChild_C|GetStaticMesh _output_get_2))))
      (Rendering|Material|SetMaterial (Variables|FocusChild_C|GetStaticMesh _output_get_2) _index (Variables|Default|GetselectionMat)))
    (if _output_get
      (Development|PrintString "FocusObject Chosen!!!!!!!!!!!!!!!!!!!!!!!")
      (bind _outactors (Actor|GetAllActorsOfClass "/Game/Blueprints/FocusParent.FocusParent_C"))
      (Input|DisableInput (Utilities|Array|Get(acopy) _outactors) _returnvalue)
      (Input|EnableInput (Game|GetPlayerCharacter 0) _returnvalue)
      (if (not (Variables|Default|GetobjDeleted))
        ;[1 1 1] Change Mesh Materials
        (for _index_2 (range 0 (Utilities|Array|Length (Rendering|Material|GetMaterials (Variables|Default|GetStaticMesh))))
          (Rendering|Material|SetMaterial (Variables|Default|GetStaticMesh) _index_2 (Utilities|Array|Get(acopy) (Variables|Default|GetoriginalMaterials) _index_2)))))))

(event Input|KeyboardEvents|Left
  (params (Key :type Key%20Structure :default "AnyKey"))
  ;[1 1 1] Legacy code
  (:Pressed
    (if (Variables|Default|GetisSelectedObject)
      _)))

(event Input|KeyboardEvents|Right
  (params (Key :type Key%20Structure :default "AnyKey"))
  ;[1 1 1] Legacy code
  (:Pressed
    (if (Variables|Default|GetisSelectedObject)
      _)))

(fn ConstructionScript
  (bind _staticmesh (Variables|Default|GetStaticMesh))
  (Components|StaticMesh|SetStaticMesh _staticmesh (Variables|Default|GetMesh))
  (Variables|Default|SetoriginalMaterials (Rendering|Material|GetMaterials _staticmesh))
  (bind _returnvalue (Rendering|Material|CreateDynamicMaterialInstance "/Game/Blueprints/FocusObject_Selection.FocusObject_Selection" :!class /Script/Engine.KismetMaterialLibrary))
  (Variables|Default|SetselectionMat _returnvalue)
  (Variables|Default|SetchildHealth (Math|Conversions|ToFloat(Integer) (Variables|Default|GetmaxHealth))))