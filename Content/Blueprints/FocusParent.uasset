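; FocusParent is a rotatable parent actor that manages which visible FocusChild actor is selected.
; Four custom events apply yaw or pitch world rotations, then line trace from the player controller toward each child component's relative location to rebuild a list of hit actors.
; Left and Right keys step a counter through that list to set IsSelectedObject, while Tick clears the flag on the other entries.
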(event Custom|rotBack
  (bind _visiblechildarray (Variables|Default|GetVisibleChildArray))
  (Utilities|FlowControl|Sequence
    (:then_0
      (Class|Actor|AddActorWorldRotation (Class|KismetMathLibrary|NegateRotator (Variables|Default|GetamountToRotate%28PITCH%29))))
    (:then_1
      (Utilities|FlowControl|Sequence
        (:then_0
          (Utilities|Array|Clear _visiblechildarray)
          (bind _output_get (Variables|Default|SetChildArray (Components|GetChildrenComponents (Variables|FocusParent_C|GetDefaultSceneRoot self) false)))
          (for _array_element _output_get
            (bind (_outhit _returnvalue) (Collision|LineTraceByChannel (Transformation|GetActorLocation (Game|GetPlayerController 0)) (Variables|/Script/Engine.SceneComponent|GetRelativeLocation _array_element) "TraceTypeQuery1" false 0 "None"))
            (if _returnvalue
              (Utilities|Array|AddUnique (Variables|Default|GetVisibleChildArray) (.HitActor (Collision|BreakHitResult _outhit)))
              (Variables|Default|SetCounter 0)))
          (for (_array_element_2 _array_index) _visiblechildarray
            (Development|PrintString (Utilities|GetDisplayName _array_element_2))
            (Development|PrintString (Utilities|String|ToString(Integer) _array_index))))))))

(event Custom|rotForward
  (bind _visiblechildarray (Variables|Default|GetVisibleChildArray))
  (Utilities|FlowControl|Sequence
    (:then_0
      (Class|Actor|AddActorWorldRotation (Variables|Default|GetamountToRotate%28YAW%29)))
    (:then_1
      (Utilities|FlowControl|Sequence
        (:then_0
          (Utilities|Array|Clear _visiblechildarray)
          (bind _output_get (Variables|Default|SetChildArray (Components|GetChildrenComponents (Variables|FocusParent_C|GetDefaultSceneRoot self) false)))
          (for _array_element _output_get
            (bind (_outhit _returnvalue) (Collision|LineTraceByChannel (Transformation|GetActorLocation (Game|GetPlayerController 0)) (Variables|/Script/Engine.SceneComponent|GetRelativeLocation _array_element) "TraceTypeQuery1" false 0 "None"))
            (if _returnvalue
              (Utilities|Array|AddUnique (Variables|Default|GetVisibleChildArray) (.HitActor (Collision|BreakHitResult _outhit)))
              (Variables|Default|SetCounter 0)))
          (for (_array_element_2 _array_index) _visiblechildarray
            (Development|PrintString (Utilities|GetDisplayName _array_element_2))
            (Development|PrintString (Utilities|String|ToString(Integer) _array_index))))))))

(event Custom|rotClock
  (bind _visiblechildarray (Variables|Default|GetVisibleChildArray))
  (Utilities|FlowControl|Sequence
    (:then_0
      (Class|Actor|AddActorWorldRotation (Class|KismetMathLibrary|NegateRotator (Variables|Default|GetamountToRotate%28YAW%29))))
    (:then_1
      (Utilities|FlowControl|Sequence
        (:then_0
          (Utilities|Array|Clear _visiblechildarray)
          (bind _output_get (Variables|Default|SetChildArray (Components|GetChildrenComponents (Variables|FocusParent_C|GetDefaultSceneRoot self) false)))
          (for _array_element _output_get
            (bind (_outhit _returnvalue) (Collision|LineTraceByChannel (Transformation|GetActorLocation (Game|GetPlayerController 0)) (Variables|/Script/Engine.SceneComponent|GetRelativeLocation _array_element) "TraceTypeQuery1" false 0 "None"))
            (if _returnvalue
              (Utilities|Array|AddUnique (Variables|Default|GetVisibleChildArray) (.HitActor (Collision|BreakHitResult _outhit)))
              (Variables|Default|SetCounter 0)))
          (for (_array_element_2 _array_index) _visiblechildarray
            (Development|PrintString (Utilities|GetDisplayName _array_element_2))
            (Development|PrintString (Utilities|String|ToString(Integer) _array_index))))))))

(event Custom|rotCountClock
  (bind _visiblechildarray (Variables|Default|GetVisibleChildArray))
  (Utilities|FlowControl|Sequence
    (:then_0
      (Class|Actor|AddActorWorldRotation (Variables|Default|GetamountToRotate%28PITCH%29)))
    (:then_1
      (Utilities|FlowControl|Sequence
        (:then_0
          (Utilities|Array|Clear _visiblechildarray)
          (bind _output_get (Variables|Default|SetChildArray (Components|GetChildrenComponents (Variables|FocusParent_C|GetDefaultSceneRoot self) false)))
          (for _array_element _output_get
            (bind (_outhit _returnvalue) (Collision|LineTraceByChannel (Transformation|GetActorLocation (Game|GetPlayerController 0)) (Variables|/Script/Engine.SceneComponent|GetRelativeLocation _array_element) "TraceTypeQuery1" false 0 "None"))
            (if _returnvalue
              (Utilities|Array|AddUnique (Variables|Default|GetVisibleChildArray) (.HitActor (Collision|BreakHitResult _outhit)))
              (Variables|Default|SetCounter 0)))
          (for (_array_element_2 _array_index) _visiblechildarray
            (Development|PrintString (Utilities|GetDisplayName _array_element_2))
            (Development|PrintString (Utilities|String|ToString(Integer) _array_index))))))))

(event Collision|EventActorBeginOverlap
  (params (OtherActor :type Actor%20Object%20Reference)))

(event EventTick
  (params (DeltaSeconds :type Float%20%28single-precision%29))
  (for (_array_element _array_index) (Variables|Default|GetVisibleChildArray)
    (bind _asfocus_child (Utilities|Casting|CastToFocusChild _array_element))
    (if (and (Variables|/Game/Blueprints/FocusChild.FocusChild_C|GetisSelectedObject _asfocus_child) (!= _array_index (Variables|Default|GetCounter)))
      (Variables|/Game/Blueprints/FocusChild.FocusChild_C|SetisSelectedObject _asfocus_child false))))

(event Input|KeyboardEvents|Right
  (params (Key :type Key%20Structure :default "AnyKey"))
  ;[1 1 1] Put in Enum to simplify/reduce code - Enum switched to equal which key was pressed, result dictates adding/subtracting from array
  (:Pressed
    (if (< (Variables|Default|GetCounter) (Utilities|Array|Length (Variables|Default|GetVisibleChildArray)))
      (bind _output_get (Variables|Default|SetCounter (+ (Variables|Default|GetCounter) 1)))
      (else
        (bind _output_get_2 (Variables|Default|SetCounter 0))))
    (bind _asfocus_child (Utilities|Casting|CastToFocusChild (Utilities|Array|Get(acopy) (Variables|Default|GetVisibleChildArray) _output_get)))
    (Variables|/Game/Blueprints/FocusChild.FocusChild_C|SetisSelectedObject _asfocus_child true)))

(event Input|KeyboardEvents|Left
  (params (Key :type Key%20Structure :default "AnyKey"))
  ;[1 1 1] Put in Enum to simplify/reduce code - Enum switched to equal which key was pressed, result dictates adding/subtracting from array
  (:Pressed
    (if (> (Variables|Default|GetCounter) 0)
      (bind _output_get (Variables|Default|SetCounter (+ (Variables|Default|GetCounter) -1)))
      (else
        (bind _output_get_2 (Variables|Default|SetCounter (Utilities|Array|Length (Variables|Default|GetVisibleChildArray))))))
    (bind _asfocus_child (Utilities|Casting|CastToFocusChild (Utilities|Array|Get(acopy) (Variables|Default|GetVisibleChildArray) _output_get)))
    (Variables|/Game/Blueprints/FocusChild.FocusChild_C|SetisSelectedObject _asfocus_child true)))

(fn ConstructionScript)