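; BP_EndPoint is a puzzle goal actor that reacts to thought bubbles overlapping it, tracking which required bubble types it has received.
; The construction script sizes a fulfilled-flag array to match Requirements, all false.
; On overlap, every unfulfilled requirement matching the bubble's Type is marked fulfilled and spawns an explosion emitter.
; Each fulfillment also raises the point light's intensity and attenuation radius by a share divided by the requirement count.
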(event Collision|EventActorBeginOverlap
  (params (OtherActor :type Actor%20Object%20Reference))
  (bind _pointlight (Variables|Default|GetPointLight))
  (bind _fulfilledrequirements (Variables|Default|GetfulfilledRequirements))
  (bind _asbp_thought_bubble (Utilities|Casting|CastToBP_ThoughtBubble OtherActor))
  (bind (_array_element _array_index) (Utilities|Array|ForEachLoopwithBreak (Variables|Default|Getrequirements))
    (:LoopBody
      (if (and (Utilities|Enum|Equal(Enum) _array_element (Variables|/Game/Puzzle_Content/Blueprints/BP_ThoughtBubble.BP_ThoughtBubble_C|Gettype _asbp_thought_bubble)) (not (Utilities|Array|Get(acopy) _fulfilledrequirements _array_index)))
        (Effects|SpawnEmitteratLocation "/Game/StarterContent/Particles/P_Explosion.P_Explosion" (Transformation|GetActorLocation))
        (Utilities|Array|SetArrayElem _fulfilledrequirements _array_index true)
        (bind _output_get (Variables|Default|SetlightIntensity (+ (Variables|Default|GetlightIntensity) (Math|Conversions|ToFloat(Integer) (/ 100000 (Utilities|Array|Length (Variables|Default|Getrequirements)))))))
        (Rendering|Components|Light|SetIntensity _pointlight _output_get)
        (bind _output_get_2 (Variables|Default|SetlightAttenuationRadius (+ (Variables|Default|GetlightAttenuationRadius) (Math|Conversions|ToFloat(Integer) (/ 1000 (Utilities|Array|Length (Variables|Default|Getrequirements)))))))
        (Rendering|Lighting|SetAttenuationRadius _pointlight _output_get_2)))))

(fn ConstructionScript
  (for _index (range 0 (- (Utilities|Array|Length (Variables|Default|Getrequirements)) 1))
    (Utilities|Array|SetArrayElem (Variables|Default|GetfulfilledRequirements) _index (Class|KismetSystemLibrary|MakeLiteralBool false) true)))