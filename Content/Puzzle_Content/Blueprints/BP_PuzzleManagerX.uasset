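; BP_PuzzleManagerX drives a thought-bubble puzzle on a fixed beat, using a Tick timer measured against SpeedOfBeats.
; On each beat it finds every BP_ThoughtBubbleX, sets its NextLocation from the NextNode of its current puzzle or spawn node target, and flags it moving.
; It then resets the timer and tells the first BP_SpawnNodeX found to spawn a new bubble.
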(event EventTick
  (params (DeltaSeconds :type Float%20%28single-precision%29))
  ;[1 1 1] Updating Thought Bubbles
  (bind _output_get (Variables|Default|Settimer (+ DeltaSeconds (Variables|Default|Gettimer))))
  (if (>= _output_get (Variables|Default|GetspeedOfBeats))
    (bind _outactors (Actor|GetAllActorsOfClass "/Game/Puzzle_Content/Blueprints/BP_ThoughtBubbleX.BP_ThoughtBubbleX_C"))
    (for _array_element _outactors
      (bind _asbp_puzzle_node_x (Utilities|Casting|CastToBP_PuzzleNodeX (Variables|/Game/Puzzle_Content/Blueprints/BP_ThoughtBubbleX.BP_ThoughtBubbleX_C|GetnextActor _array_element))
        (:then
          (Variables|/Game/Puzzle_Content/Blueprints/BP_ThoughtBubbleX.BP_ThoughtBubbleX_C|SetnextLocation _array_element (Variables|/Game/Puzzle_Content/Blueprints/BP_PuzzleNodeX.BP_PuzzleNodeX_C|GetnextNode _asbp_puzzle_node_x)))
        (:CastFailed
          (bind _asbp_spawn_node_x (Utilities|Casting|CastToBP_SpawnNodeX (Variables|/Game/Puzzle_Content/Blueprints/BP_ThoughtBubbleX.BP_ThoughtBubbleX_C|GetnextActor _array_element)))
          (Variables|/Game/Puzzle_Content/Blueprints/BP_ThoughtBubbleX.BP_ThoughtBubbleX_C|SetnextLocation _array_element (Variables|/Game/Puzzle_Content/Blueprints/BP_SpawnNodeX.BP_SpawnNodeX_C|GetnextNode _asbp_spawn_node_x))))
      (Variables|/Game/Puzzle_Content/Blueprints/BP_ThoughtBubbleX.BP_ThoughtBubbleX_C|Setmoving _array_element true))
    (Variables|Default|Settimer 0.0)
    ;[1 1 1] Spawn Bubbles
    (bind _outactors_2 (Actor|GetAllActorsOfClass "/Game/Puzzle_Content/Blueprints/BP_SpawnNodeX.BP_SpawnNodeX_C"))
    (Default|SpawnBubble (Utilities|Array|Get(acopy) _outactors_2))))

(fn ConstructionScript)