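; BP_PuzzleNode is a clickable puzzle waypoint that holds a list of connected nodes and selects one of them as the next destination.
; The construction script and BeginPlay aim its Arrow at the first node, with BeginPlay also storing that location as NextNode.
; Clicking cycles through the list with wraparound when several nodes exist, updating NextNode and rotating the Arrow to face it.
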(event EventBeginPlay
  ;[1 1 1] Setting the default Next Node
  (bind _output_get (Variables|Default|SetnextNode (Transformation|GetActorLocation (Utilities|Array|Get(acopy) (Variables|Default|GetNodes)))))
  (Transformation|SetWorldRotation (Variables|Components|GetArrow) (Math|Rotator|FindLookatRotation (Transformation|GetActorLocation) _output_get) false false))

(event MouseInput|EventActorOnClicked
  (params (ButtonPressed :type Key%20Structure :default "AnyKey"))
  (bind _nodes (Variables|Default|GetNodes))
  (bind _returnvalue (Utilities|Array|Length _nodes))
  ;[1 1 1] Switch Directions
  (if (> _returnvalue 1)
    (bind _output_get (Variables|Default|SetcurrentArrayIndex (+ (Variables|Default|GetcurrentArrayIndex) 1)))
    (if (>= _output_get _returnvalue)
      (Variables|Default|SetcurrentArrayIndex 0))
    (bind _output_get_2 (Variables|Default|SetnextNode (Transformation|GetActorLocation (Utilities|Array|Get(acopy) (Variables|Default|GetNodes) (Variables|Default|GetcurrentArrayIndex)))))
    (Transformation|SetWorldRotation (Variables|Components|GetArrow) (Math|Rotator|FindLookatRotation (Transformation|GetActorLocation) _output_get_2) false false)))

(fn ConstructionScript
  (Transformation|SetWorldRotation (Variables|Components|GetArrow) (Math|Rotator|FindLookatRotation (Transformation|GetActorLocation) (Transformation|GetActorLocation (Utilities|Array|Get(acopy) (Variables|Default|GetNodes)))) false false))