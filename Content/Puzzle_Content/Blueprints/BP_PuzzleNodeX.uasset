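; Clickable neuron junction for a puzzle that holds a switchable next-node location among its linked Nodes.
; Clicking cycles the target and re-aims the Arrow, while the construction script adds an arrow toward each linked node.
; Tick shows an Indicator when the cursor is near the junction on screen and multiple exits exist.
; An overlapping BP_ThoughtBubbleX tints the mesh red, blue or green by Type until it leaves.
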(event EventBeginPlay
  ;[1 1 1] Setting the default Next Node
  (bind _output_get (Variables|Default|SetnextNode (Transformation|GetActorLocation (Utilities|Array|Get(acopy) (Variables|Default|GetNodes)))))
  (Transformation|SetWorldRotation (Variables|Components|GetArrow) (Math|Rotator|FindLookatRotation (Transformation|GetActorLocation) _output_get) false false))

(event MouseInput|EventActorOnClicked
  (params (ButtonPressed :type Key%20Structure :default "AnyKey"))
  (bind _nodes (Variables|Default|GetNodes))
  (bind _returnvalue (Utilities|Array|Length _nodes))
  ;[1 1 1] Switch Directions
  (if (> _returnvalue 1)
    (bind _output_get (Variables|Default|SetcurrentArrayIndex (+ (Variables|Default|GetcurrentArrayIndex) 1)))
    (if (>= _output_get _returnvalue)
      (Variables|Default|SetcurrentArrayIndex 0))
    (bind _output_get_2 (Variables|Default|SetnextNode (Transformation|GetActorLocation (Utilities|Array|Get(acopy) (Variables|Default|GetNodes) (Variables|Default|GetcurrentArrayIndex)))))
    (Transformation|SetWorldRotation (Variables|Components|GetArrow) (Math|Rotator|FindLookatRotation (Transformation|GetActorLocation) _output_get_2) false false)))

(event EventTick
  (params (DeltaSeconds :type Float%20%28single-precision%29))
  (bind _returnvalue (Game|GetPlayerController 0))
  (bind _indicator (Variables|Default|GetIndicator))
  (bind (_locationx _locationy) (Game|Player|GetMousePosition _returnvalue))
  ;[1 1 1] Mouse Indicator When Nearby
  (if (and (< (Math|Vector|VectorLength (- (Math|Conversions|ToVector(Vector2D) (.ScreenPosition (Class|GameplayStatics|ProjectWorldtoScreen _returnvalue (Transformation|GetActorLocation)))) (Math|Conversions|ToVector(Vector2D) (Math|Vector2D|MakeVector2D _locationx _locationy)))) 5e+01) (> (Utilities|Array|Length (Variables|Default|GetNodes)) 1))
    (Rendering|SetVisibility _indicator true false)
    (else
      (Rendering|SetVisibility _indicator false false))))

(event Collision|EventActorBeginOverlap
  (params (OtherActor :type Actor%20Object%20Reference))
  ;[1 1 1] Changing material when overlapped
  (bind _asbp_thought_bubble_x (Utilities|Casting|CastToBP_ThoughtBubbleX OtherActor))
  (Variables|Default|Setoverlapped _asbp_thought_bubble_x)
  (if (Utilities|Enum|Equal(Enum) (Variables|/Game/Puzzle_Content/Blueprints/BP_ThoughtBubbleX.BP_ThoughtBubbleX_C|Gettype _asbp_thought_bubble_x) "red")
    (bind _returnvalue (Rendering|Material|CreateDynamicMaterialInstance (Variables|Components|GetMesh) 0 "/Game/Puzzle_Content/Materials/M_NeuronJunction.M_NeuronJunction" :!class /Script/Engine.PrimitiveComponent))
    (Rendering|Material|SetVectorParameterValue _returnvalue "BaseColor" "(R=0.960000,G=0.000000,B=0.077504,A=1.000000)" :!class /Script/Engine.MaterialInstanceDynamic)
    (elif (Utilities|Enum|Equal(Enum) (Variables|/Game/Puzzle_Content/Blueprints/BP_ThoughtBubbleX.BP_ThoughtBubbleX_C|Gettype _asbp_thought_bubble_x) "blue")
      (bind _returnvalue_2 (Rendering|Material|CreateDynamicMaterialInstance (Variables|Components|GetMesh) 0 "/Game/Puzzle_Content/Materials/M_NeuronJunction.M_NeuronJunction" :!class /Script/Engine.PrimitiveComponent))
      (Rendering|Material|SetVectorParameterValue _returnvalue_2 "BaseColor" "(R=0.068933,G=0.305205,B=0.960000,A=1.000000)" :!class /Script/Engine.MaterialInstanceDynamic)
      (elif (Utilities|Enum|Equal(Enum) (Variables|/Game/Puzzle_Content/Blueprints/BP_ThoughtBubbleX.BP_ThoughtBubbleX_C|Gettype _asbp_thought_bubble_x) "green")
        (bind _returnvalue_3 (Rendering|Material|CreateDynamicMaterialInstance (Variables|Components|GetMesh) 0 "/Game/Puzzle_Content/Materials/M_NeuronJunction.M_NeuronJunction" :!class /Script/Engine.PrimitiveComponent))
        (Rendering|Material|SetVectorParameterValue _returnvalue_3 "BaseColor" "(R=0.116486,G=0.710000,B=0.030146,A=1.000000)" :!class /Script/Engine.MaterialInstanceDynamic)))))

(event Collision|EventActorEndOverlap
  (params (OtherActor :type Actor%20Object%20Reference))
  (if (== OtherActor (Variables|Default|Getoverlapped))
    (Rendering|Material|SetMaterial (Variables|Components|GetMesh) 0 "/Game/Puzzle_Content/Materials/M_NeuronJunction.M_NeuronJunction")))

(fn ConstructionScript
  (Transformation|SetWorldRotation (Variables|Components|GetArrow) (Math|Rotator|FindLookatRotation (Transformation|GetActorLocation) (Transformation|GetActorLocation (Utilities|Array|Get(acopy) (Variables|Default|GetNodes)))) false false)
  (for _array_element (Variables|Default|GetNodes)
    (AddComponent|AddArrowComponent false (Math|Transform|MakeTransform "0,0.000000,50.000000" (Math|Rotator|FindLookatRotation (Transformation|GetActorLocation) (Transformation|GetActorLocation _array_element))))))