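; BP_SpawnNode is a puzzle start node that spawns thought bubbles and sends them toward one of its linked Nodes.
; Clicking it cycles NextNode through the linked nodes and turns the main Arrow to show the chosen direction.
; The construction script adds an arrow toward each linked node as a path preview.
; SpawnBubble advances through the Bubbles type list, spawning BP_ThoughtBubble above the node and starting it moving toward NextNode.
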(event EventBeginPlay
  ;[1 1 1] Setting the default Next Node
  (bind _output_get (Variables|Default|SetnextNode (Transformation|GetActorLocation (Utilities|Array|Get(acopy) (Variables|Default|GetNodes)))))
  (Transformation|SetWorldRotation (Variables|Default|GetArrow) (Math|Rotator|FindLookatRotation (Transformation|GetActorLocation) _output_get) false false))

(event MouseInput|EventActorOnClicked
  (params (ButtonPressed :type Key%20Structure :default "AnyKey"))
  (bind _nodes (Variables|Default|GetNodes))
  (bind _returnvalue (Utilities|Array|Length _nodes))
  ;[1 1 1] Switch Directions
  (if (> _returnvalue 1)
    (bind _output_get (Variables|Default|SetcurrentArrayIndex (+ (Variables|Default|GetcurrentArrayIndex) 1)))
    (if (>= _output_get _returnvalue)
      (Variables|Default|SetcurrentArrayIndex 0))
    (bind _output_get_2 (Variables|Default|SetnextNode (Transformation|GetActorLocation (Utilities|Array|Get(acopy) (Variables|Default|GetNodes) (Variables|Default|GetcurrentArrayIndex)))))
    (Transformation|SetWorldRotation (Variables|Default|GetArrow) (Math|Rotator|FindLookatRotation (Transformation|GetActorLocation) _output_get_2) false false)))

(fn ConstructionScript
  (Transformation|SetWorldRotation (Variables|Default|GetArrow) (Math|Rotator|FindLookatRotation (Transformation|GetActorLocation) (Transformation|GetActorLocation (Utilities|Array|Get(acopy) (Variables|Default|GetNodes)))) false false)
  (for _array_element (Variables|Default|GetNodes)
    (AddComponent|AddArrowComponent false (Math|Transform|MakeTransform "0,0.000000,50.000000" (Math|Rotator|FindLookatRotation (Transformation|GetActorLocation) (Transformation|GetActorLocation _array_element))))))

(fn SpawnBubble
  (bind _result (Math|Integer|IncrementInt (Variables|Default|GetcurrentIndex))
    (:%20%20
      (if (< _result (Utilities|Array|Length (Variables|Default|GetBubbles)))
        (bind _returnvalue (Game|SpawnActorfromClass "/Game/Puzzle_Content/Blueprints/BP_ThoughtBubble.BP_ThoughtBubble_C" (Math|Transform|MakeTransform (+ (Transformation|GetActorLocation) "0, 0,100.000000")) "Undefined" 0 self (Utilities|Array|Get(acopy) (Variables|Default|GetBubbles) (Variables|Default|GetcurrentIndex))))
        (bind _asbp_puzzle_node (Utilities|Casting|CastToBP_PuzzleNode (Variables|/Game/Puzzle_Content/Blueprints/BP_ThoughtBubble.BP_ThoughtBubble_C|GetnextPosition _returnvalue))
          (:then
            (Variables|/Game/Puzzle_Content/Blueprints/BP_ThoughtBubble.BP_ThoughtBubble_C|SetnextLocation _returnvalue (Variables|/Game/Puzzle_Content/Blueprints/BP_PuzzleNode.BP_PuzzleNode_C|GetnextNode _asbp_puzzle_node)))
          (:CastFailed
            (bind _asbp_spawn_node (Utilities|Casting|CastToBP_SpawnNode (Variables|/Game/Puzzle_Content/Blueprints/BP_ThoughtBubble.BP_ThoughtBubble_C|GetnextPosition _returnvalue)))
            (Variables|/Game/Puzzle_Content/Blueprints/BP_ThoughtBubble.BP_ThoughtBubble_C|SetnextLocation _returnvalue (Variables|BP_SpawnNode_C|GetnextNode _asbp_spawn_node))))
        (Variables|/Game/Puzzle_Content/Blueprints/BP_ThoughtBubble.BP_ThoughtBubble_C|Setmoving _returnvalue true)))))