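; BP_ThoughtBubble is a puzzle bubble whose Type sets a red, blue or green material and light color.
; When Moving is set, a timeline drives Move, lerping it to hover above NextLocation with sweep while the mesh shrinks and regrows.
; Overlaps store puzzle or spawn nodes as NextActor; endpoints remove the bubble from Manager and destroy it after a delay, while other bubbles trigger an explosion and immediate removal.
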(event Collision|EventActorBeginOverlap
  (params (OtherActor :type Actor%20Object%20Reference))
  ;[1 1 1] Collision
  (bind _asbp_puzzle_node (Utilities|Casting|CastToBP_PuzzleNode OtherActor)
    (:then
      (Variables|Default|SetnextActor _asbp_puzzle_node))
    (:CastFailed
      (Utilities|Casting|CastToBP_EndPoint OtherActor
        (:then
          (Utilities|FlowControl|Delay 0.2)
          (Utilities|Array|RemoveItem (Variables|/Game/Puzzle_Content/Blueprints/BP_PuzzleManager.BP_PuzzleManager_C|GetthoughtBubbles (Variables|Default|Getmanager)) self :!label _label)
          (Actor|DestroyActor))
        (:CastFailed
          (Utilities|Casting|CastToBP_ThoughtBubble OtherActor
            (:then
              (Effects|SpawnEmitteratLocation "/Game/StarterContent/Particles/P_Explosion.P_Explosion" (Transformation|GetActorLocation))
              (goto _label))
            (:CastFailed
              (bind _asbp_spawn_node (Utilities|Casting|CastToBP_SpawnNode OtherActor))
              (Variables|Default|SetnextActor _asbp_spawn_node))))))))

(event EventTick
  (params (DeltaSeconds :type Float%20%28single-precision%29))
  ;[1 1 1] Movement
  (if (Variables|Default|Getmoving)
    (bind _alpha (Timeline|Timeline_0 PlayFromStart)
      (:Update
        (CallFunction|Move _alpha)
        (Variables|Default|Setmoving false))
      (:Finished
        (Transformation|SetWorldScale3D (Variables|Default|GetMesh) "1.000000,1.000000,1.000000")))))

(fn ConstructionScript
  (Utilities|FlowControl|Sequence
    (:then_0
      (if (Utilities|Enum|Equal(Enum) (Variables|Default|Gettype) "red")
        (Rendering|Material|SetMaterial (Variables|Default|GetMesh) 0 "/Game/Puzzle_Content/Materials/M_RedBubble.M_RedBubble")
        (Rendering|Components|Light|SetLightColor (Variables|Default|GetPointLight) "(R=1.000000,G=0.405000,B=0.567530,A=1.000000)" true)))
    (:then_1
      (if (Utilities|Enum|Equal(Enum) (Variables|Default|Gettype) "blue")
        (Rendering|Material|SetMaterial (Variables|Default|GetMesh) 0 "/Game/Puzzle_Content/Materials/M_BlueBubble.M_BlueBubble")
        (Rendering|Components|Light|SetLightColor (Variables|Default|GetPointLight) "(R=0.000000,G=0.821918,B=1.000000,A=1.000000)" true)))
    (:then_2
      (if (Utilities|Enum|Equal(Enum) (Variables|Default|Gettype) "green")
        (Rendering|Material|SetMaterial (Variables|Default|GetMesh) 0 "/Game/Puzzle_Content/Materials/M_GreenBubble.M_GreenBubble")
        (Rendering|Components|Light|SetLightColor (Variables|Default|GetPointLight) "(R=0.007687,G=1.000000,B=0.000000,A=1.000000)" true)))))

(fn Move
  (params (Alpha :type Float%20%28single-precision%29))
  ;[1 1 1] Lerping Location
  (Transformation|SetActorLocation (Math|Vector|Lerp(Vector) (Transformation|GetActorLocation) (+ (Variables|Default|GetnextLocation) "0.000000,0.000000,50.000000") Alpha) true false)
  ;[1 1 1] Lerping Size
  (if (and (> Alpha 0.1) (< Alpha 0.4))
    (if (> (.X (Math|Vector|BreakVector (Variables|Default|Getscale))) 0.3)
      (bind _output_get (Variables|Default|Setscale (- (Variables|Default|Getscale) "0.100000,0.100000,0.100000")))
      (Transformation|SetWorldScale3D (Variables|Default|GetMesh) _output_get))
    (elif (< (.X (Math|Vector|BreakVector (Variables|Default|Getscale))) 1.0)
      (bind _output_get_2 (Variables|Default|Setscale (+ (Variables|Default|Getscale) "0.100000,0.100000,0.100000")))
      (Transformation|SetWorldScale3D (Variables|Default|GetMesh) _output_get_2))))