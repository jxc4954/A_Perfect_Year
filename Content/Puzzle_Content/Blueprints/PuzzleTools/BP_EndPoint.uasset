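; Puzzle goal actor that checks overlapping BP_ThoughtBubbleX types against its colour Requirements and completes the puzzle when all are fulfilled.
; The construction script builds five spotlights, showing and colouring a two- or three-light set to match the requirements.
; Each match spawns an explosion and brightens its light.
; Completion notifies the Manager, restores player movement and camera, then destroys the puzzle camera; the created win screen is never displayed.
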(event Collision|EventActorBeginOverlap
  (params (OtherActor :type Actor%20Object%20Reference))
  (bind _manager (Variables|Default|Getmanager))
  (bind _spotlights (Variables|Default|GetSpotLights))
  (bind _fulfilledrequirements (Variables|Default|GetfulfilledRequirements))
  (bind _asbp_thought_bubble_x (Utilities|Casting|CastToBP_ThoughtBubbleX OtherActor))
  (bind (_array_element _array_index) (Utilities|Array|ForEachLoopwithBreak (Variables|Default|Getrequirements) :!label _label)
    (:LoopBody
      (if (and (Utilities|Enum|Equal(Enum) _array_element (Variables|/Game/Puzzle_Content/Blueprints/BP_ThoughtBubbleX.BP_ThoughtBubbleX_C|Gettype _asbp_thought_bubble_x)) (not (Utilities|Array|Get(acopy) _fulfilledrequirements _array_index)))
        (Math|Integer|IncrementInt (Variables|Default|GetrequirementIterator)
          (:%20%20
            (Effects|SpawnEmitteratLocation "/Game/StarterContent/Particles/P_Explosion.P_Explosion" (Transformation|GetActorLocation))
            (Utilities|Array|SetArrayElem _fulfilledrequirements _array_index true)
            (if (== (Utilities|Array|Length (Variables|Default|Getrequirements)) 2)
              (Rendering|Components|Light|SetIntensity (Utilities|Array|Get(acopy) _spotlights _array_index) 5e+04)
              (else
                (Rendering|Components|Light|SetIntensity (Utilities|Array|Get(acopy) _spotlights (+ _array_index 2)) 5e+04)))
            (if (== (Variables|Default|GetnumRequirements) (Variables|Default|GetrequirementIterator))
              (Variables|/Game/Puzzle_Content/Blueprints/PuzzleBlueprints/BP_PuzzleManager.BP_PuzzleManager_C|SetisWon _manager true)
              (Default|DestroyPuzzle _manager)
              ;[1 1 1] Allowing player to move again
              (bind _outactors (Actor|GetAllActorsOfClass "/Game/Runner_Content/Blueprints/BP_Player.BP_Player_C"))
              (Variables|/Game/Runner_Content/Blueprints/BP_Player.BP_Player_C|SetCanMove (Utilities|Array|Get(acopy) _outactors) true)
              (Variables|/Script/Engine.CharacterMovementComponent|SetGravityScale (Variables|/Script/Engine.Character|GetCharacterMovement (Utilities|Array|Get(acopy) _outactors)) 1.0)
              ;[1 1 1] Moving back to player camera
              (bind _outactors_2 (Actor|GetAllActorsOfClass "/Game/Runner_Content/Blueprints/BP_Player.BP_Player_C"))
              (Utilities|FlowControl|Delay 1.0)
              (Components|Activation|Activate (Variables|/Game/Runner_Content/Blueprints/BP_Player.BP_Player_C|GetPlayerCam (Utilities|Array|Get(acopy) _outactors_2)) false)
              (Components|Activation|Deactivate (Variables|/Game/Runner_Content/Blueprints/BP_Player.BP_Player_C|GetPuzzleCamera (Utilities|Array|Get(acopy) _outactors_2)))
              (bind _outactors_3 (Actor|GetAllActorsOfClass "/Game/Puzzle_Content/Blueprints/BP_PuzzleCamera.BP_PuzzleCamera_C"))
              (Actor|DestroyActor (Utilities|Array|Get(acopy) _outactors_3))
              (else
                (goto _label Break)))))))))

(event EventBeginPlay
  (bind _returnvalue (UserInterface|CreateWidget "/Game/Puzzle_Content/Widgets/W_WinScreen.W_WinScreen_C"))
  (Variables|Default|SetwinScreenRef _returnvalue)
  (bind _outactors (Actor|GetAllActorsOfClass "/Game/Puzzle_Content/Blueprints/BP_PuzzleCamera.BP_PuzzleCamera_C"))
  (bind _output_get (Variables|Default|SetcamRef (Utilities|Array|Get(acopy) _outactors)))
  (Variables|Default|SetcamLoc (Transformation|GetActorLocation _output_get)))

(fn ConstructionScript
  (bind _spotlights (Variables|Default|GetSpotLights))
  (bind _requirements (Variables|Default|Getrequirements))
  (bind _returnvalue (Utilities|Array|Length _requirements))
  (for _index (range 0 4)
    (bind _returnvalue_2 (AddComponent|AddSpotLightComponent false (Utilities|Array|Get(acopy) (Variables|Default|GetlightTransformArr) _index)))
    (bind _returnvalue_3 (Utilities|Array|Add _spotlights _returnvalue_2))
    (Rendering|Lighting|SetAttenuationRadius (Utilities|Array|Get(acopy) _spotlights _returnvalue_3) (Variables|Default|GetlightAttenuationRadius))
    (Rendering|Components|Light|SetIntensity (Utilities|Array|Get(acopy) _spotlights _returnvalue_3) (Variables|Default|GetlightIntensity))
    (if (< _index 2)
      (Rendering|Lighting|SetInnerConeAngle (Utilities|Array|Get(acopy) _spotlights _returnvalue_3) 8e+01)
      (else
        (Rendering|Lighting|SetInnerConeAngle (Utilities|Array|Get(acopy) _spotlights _returnvalue_3) 6e+01))))
  ;[1 1 1] Setting Requirements
  (Variables|Default|SetnumRequirements _returnvalue)
  (for _index_2 (range 0 (- _returnvalue 1))
    (Utilities|Array|SetArrayElem (Variables|Default|GetfulfilledRequirements) _index_2 (Class|KismetSystemLibrary|MakeLiteralBool false) true))
  ;[1 1 1] Changing Light Color Depending on Requirements
  (Utilities|FlowControl|Sequence
    (:then_0
      (if (== _returnvalue 2)
        (for (_array_element _array_index) (Variables|Default|GetSpotLights)
          (if (< _array_index 2)
            (Rendering|SetVisibility _array_element true false)
            (if (Utilities|Enum|Equal(Enum) (Utilities|Array|Get(acopy) (Variables|Default|Getrequirements) _array_index) "red")
              (Rendering|Components|Light|SetLightColor _array_element (Utilities|Array|Get(acopy) (Variables|Default|GetcolorArr)) true)
              (elif (Utilities|Enum|Equal(Enum) (Utilities|Array|Get(acopy) (Variables|Default|Getrequirements) _array_index) "blue")
                (Rendering|Components|Light|SetLightColor _array_element (Utilities|Array|Get(acopy) (Variables|Default|GetcolorArr) 1) true)
                (elif (Utilities|Enum|Equal(Enum) (Utilities|Array|Get(acopy) (Variables|Default|Getrequirements) _array_index) "green")
                  (Rendering|Components|Light|SetLightColor _array_element (Utilities|Array|Get(acopy) (Variables|Default|GetcolorArr) 2) true))))
            (else
              (Rendering|SetVisibility _array_element false false))))))
    (:then_1
      (if (== _returnvalue 3)
        (for (_array_element_2 _array_index_2) (Variables|Default|GetSpotLights)
          (if (> _array_index_2 1)
            (Rendering|SetVisibility _array_element_2 true false)
            (if (Utilities|Enum|Equal(Enum) (Utilities|Array|Get(acopy) (Variables|Default|Getrequirements) (- _array_index_2 2)) "red")
              (Rendering|Components|Light|SetLightColor _array_element_2 (Utilities|Array|Get(acopy) (Variables|Default|GetcolorArr)) true)
              (elif (Utilities|Enum|Equal(Enum) (Utilities|Array|Get(acopy) (Variables|Default|Getrequirements) (- _array_index_2 2)) "blue")
                (Rendering|Components|Light|SetLightColor _array_element_2 (Utilities|Array|Get(acopy) (Variables|Default|GetcolorArr) 1) true)
                (elif (Utilities|Enum|Equal(Enum) (Utilities|Array|Get(acopy) (Variables|Default|Getrequirements) (- _array_index_2 2)) "green")
                  (Rendering|Components|Light|SetLightColor _array_element_2 (Utilities|Array|Get(acopy) (Variables|Default|GetcolorArr) 2) true))))
            (else
              (Rendering|SetVisibility _array_element_2 false false))))))))