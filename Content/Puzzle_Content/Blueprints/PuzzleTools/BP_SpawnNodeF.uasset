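; Puzzle spawn node that releases thought bubbles and sends them toward a player-selectable next node.
; Clicking cycles the target through its node list and rotates the arrow to face it; SetArrows adds an arrow per branch when several exist.
; Each SpawnBubble call spawns the next typed bubble from the list, registers it with the manager and starts it moving, flagging DoneSpawning once the list runs out.
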(event EventBeginPlay
  ;[1 1 1] Setting the default Next Node
  (bind _output_get (Variables|Default|SetnextNode (Utilities|Array|Get(acopy) (Variables|Default|GetNodes))))
  (Transformation|SetWorldRotation (Variables|Default|GetArrow) (Math|Rotator|FindLookatRotation (Transformation|GetActorLocation) _output_get) false false))

(event MouseInput|EventActorOnClicked
  (params (ButtonPressed :type Key%20Structure :default "AnyKey"))
  (bind _nodes (Variables|Default|GetNodes))
  (bind _returnvalue (Utilities|Array|Length _nodes))
  ;[1 1 1] Switch Directions
  (if (> _returnvalue 1)
    (bind _output_get (Variables|Default|SetcurrentArrayIndex (+ (Variables|Default|GetcurrentArrayIndex) 1)))
    (if (>= _output_get _returnvalue)
      (Variables|Default|SetcurrentArrayIndex 0))
    (bind _output_get_2 (Variables|Default|SetnextNode (Utilities|Array|Get(acopy) (Variables|Default|GetNodes) (Variables|Default|GetcurrentArrayIndex))))
    (Transformation|SetWorldRotation (Variables|Default|GetArrow) (Math|Rotator|FindLookatRotation (Transformation|GetActorLocation) _output_get_2) false false)))

(fn ConstructionScript)

(fn SpawnBubble
  (bind _returnvalue (Transformation|GetActorLocation))
  (bind _result (Math|Integer|IncrementInt (Variables|Default|GetcurrentIndex))
    (:%20%20
      (if (< _result (Utilities|Array|Length (Variables|Default|GetBubbles)))
        (bind _returnvalue_2 (Game|SpawnActorfromClass "/Game/Puzzle_Content/Blueprints/BP_ThoughtBubbleX.BP_ThoughtBubbleX_C" (Math|Transform|MakeTransform (+ _returnvalue (* (* (Math|Vector|Normalize (- _returnvalue (Variables|Default|GetnextNode))) 1.0) (Variables|Default|GetpuzzleScale))) "0, 0, 0" (Variables|Default|GetpuzzleScale)) "Undefined" 0 self (Utilities|Array|Get(acopy) (Variables|Default|GetBubbles) (Variables|Default|GetcurrentIndex)) (Variables|Default|Getmanager) (Variables|Default|GetpuzzleScale)))
        (Utilities|Array|Add (Variables|/Game/Puzzle_Content/Blueprints/PuzzleBlueprints/BP_PuzzleManager.BP_PuzzleManager_C|GetthoughtBubbles (Variables|Default|Getmanager)) _returnvalue_2)
        (bind _asbp_puzzle_node (Utilities|Casting|CastToBP_PuzzleNode (Variables|/Game/Puzzle_Content/Blueprints/BP_ThoughtBubbleX.BP_ThoughtBubbleX_C|GetnextActor _returnvalue_2))
          (:then
            (Variables|/Game/Puzzle_Content/Blueprints/BP_ThoughtBubbleX.BP_ThoughtBubbleX_C|SetnextLocation _returnvalue_2 (Variables|/Game/Puzzle_Content/Blueprints/PuzzleTools/BP_PuzzleNode.BP_PuzzleNode_C|GetnextNode _asbp_puzzle_node)))
          (:CastFailed
            (bind _asbp_spawn_node_f (Utilities|Casting|CastToBP_SpawnNodeF (Variables|/Game/Puzzle_Content/Blueprints/BP_ThoughtBubbleX.BP_ThoughtBubbleX_C|GetnextActor _returnvalue_2)))
            (Variables|/Game/Puzzle_Content/Blueprints/BP_ThoughtBubbleX.BP_ThoughtBubbleX_C|SetnextLocation _returnvalue_2 (Variables|BP_SpawnNodeF_C|GetnextNode _asbp_spawn_node_f))))
        (Variables|/Game/Puzzle_Content/Blueprints/BP_ThoughtBubbleX.BP_ThoughtBubbleX_C|Setmoving _returnvalue_2 true)
        (else
          (Variables|Default|SetdoneSpawning true))))))

(fn SetArrows
  (Transformation|SetWorldRotation (Variables|Default|GetArrow) (Math|Rotator|FindLookatRotation (Transformation|GetActorLocation) (Utilities|Array|Get(acopy) (Variables|Default|GetNodes))) false false)
  (if (> (Utilities|Array|Length (Variables|Default|GetNodes)) 1)
    (for _array_element (Variables|Default|GetNodes)
      (bind _returnvalue (AddComponent|AddArrowComponent false (Math|Transform|MakeTransform "0, 0,50.000000")))
      (Transformation|SetWorldRotation _returnvalue (Math|Rotator|FindLookatRotation (Transformation|GetActorLocation) _array_element) false false))))