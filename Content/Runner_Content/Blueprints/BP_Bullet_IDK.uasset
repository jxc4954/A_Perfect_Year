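; BP_Bullet_IDK is a projectile actor that destroys itself when its static mesh hits the player character or a bullet wall.
; Every hit also draws a short-lived red debug sphere at the impact point, and no damage is applied.
; InitVelocity launches it by passing the spawn forward vector times speed to ProjectileMovement as a local-space velocity, leaving the spawn location input unused.
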(event OnComponentHit(StaticMesh)
  (params (HitComponent :type Primitive%20Component%20Object%20Reference) (OtherActor :type Actor%20Object%20Reference) (OtherComp :type Primitive%20Component%20Object%20Reference) (NormalImpulse :type Vector :default "0, 0, 0") (Hit :type Hit%20Result%20Structure%20%28by%20ref%29))
  ;[1 1 1] Self-Destruct on Hit
  (if (or (== (Utilities|GetClass OtherActor) "/Game/ThirdPersonBP/Blueprints/BP_PlayerCharacter.BP_PlayerCharacter_C") (== (Utilities|GetClass OtherActor) "/Game/RPG_Content/BattleSystem/BP_BulletWall.BP_BulletWall_C"))
    (Actor|DestroyActor))
  (Rendering|Debug|DrawDebugSphere (.Location (Collision|BreakHitResult Hit)) 12.0 12 "(R=1.000000,G=0.009454,B=0.000000,A=1.000000)" 2.0 2.0))

(event EventTick
  (params (DeltaSeconds :type Float%20%28single-precision%29)))

(fn ConstructionScript)

(fn InitVelocity
  (params (SpawnLoc :type Vector) (SpawnForward :type Vector) (Speed :type Float%20%28single-precision%29))
  (Game|Components|ProjectileMovement|SetVelocityinLocalSpace (Variables|Default|GetProjectileMovement) (* SpawnForward Speed)))