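; Corner tile for an endless runner's tunnel that turns the track.
; BeginPlay spawns a BP_TurnTrigger ahead of the tile.
; When BP_Player overlaps its box, it asks BP_RunnerMode for the next tunnel tile, then destroys itself after a delay.
; GetAttachTransform randomly rolls the corner upside down (one in four) to flip the turn direction before returning the AttachPoint transform.
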(event OnComponentBeginOverlap(Box)
  (params (OverlappedComponent :type Primitive%20Component%20Object%20Reference) (OtherActor :type Actor%20Object%20Reference) (OtherComp :type Primitive%20Component%20Object%20Reference) (OtherBodyIndex :type Integer) (bFromSweep :type Boolean) (SweepResult :type Hit%20Result%20Structure%20%28by%20ref%29))
  ;[1 1 1] Spawn Next Tile and Self-Destruct
  (Utilities|Casting|CastToBP_Player OtherActor)
  (bind _asbp_runner_mode (Utilities|Casting|CastToBP_RunnerMode (Game|GetGameMode)))
  (Default|SpawnTunnelTile _asbp_runner_mode)
  (Utilities|FlowControl|Delay 1e+01)
  (Actor|DestroyActor))

(event EventBeginPlay
  (bind _returnvalue (Transformation|GetActorTransform))
  ;[1 1 1] Spawn Turn Trigger
  (Game|SpawnActorfromClass "/Game/Runner_Content/Blueprints/BP_TurnTrigger.BP_TurnTrigger_C" (Math|Transform|MakeTransform (+ (.location _returnvalue) (* (Transformation|GetActorForwardVector) 1e+03)) (.rotation _returnvalue) (.scale _returnvalue)) "Undefined" 0 0))

(event Collision|EventActorBeginOverlap
  (params (OtherActor :type Actor%20Object%20Reference)))

(event EventTick
  (params (DeltaSeconds :type Float%20%28single-precision%29)))

(fn ConstructionScript)

(fn GetAttachTransform
  (CallFunction|RandomRotation)
  (return (Transformation|GetWorldTransform (Variables|Default|GetAttachPoint))))

(fn RandomRotation
  (bind _returnvalue (Transformation|GetActorRotation))
  (switch int (Math|Random|RandomIntegerinRange 0 3)
    (:Default
      (Transformation|SetActorRotation (Math|Rotator|CombineRotators (Math|Rotator|MakeRotator 0.0 0.0 0.0) _returnvalue) :!label _label))
    (:0
      (goto _label))
    (:1
      (Transformation|SetActorRotation (Math|Rotator|CombineRotators (Math|Rotator|MakeRotator 1.8e+02 0.0 0.0) _returnvalue)))))