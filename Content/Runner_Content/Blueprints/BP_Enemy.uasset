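; BP_Enemy is a shooting enemy that destroys itself when its cube is hit by a BP_Bullet.
; Tick accumulates time, fires at RateOfFire and flips direction, sliding along world X only during the last half second before each shot.
; Shoot spawns a short-lived bullet rotated toward the first BP_Player found.
; The GetForward vector feeds only a disconnected InitVelocity call, so it has no effect.
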(event OnComponentHit(Cube)
  (params (HitComponent :type Primitive%20Component%20Object%20Reference) (OtherActor :type Actor%20Object%20Reference) (OtherComp :type Primitive%20Component%20Object%20Reference) (NormalImpulse :type Vector :default "0, 0, 0") (Hit :type Hit%20Result%20Structure%20%28by%20ref%29))
  ;[1 1 1] Self-Destruct on Bullet Hit
  (Utilities|Casting|CastToBP_Bullet OtherActor)
  (Actor|DestroyActor))

(event EventBeginPlay)

(event Collision|EventActorBeginOverlap
  (params (OtherActor :type Actor%20Object%20Reference)))

(event EventTick
  (params (DeltaSeconds :type Float%20%28single-precision%29))
  (bind _returnvalue (Transformation|GetActorLocation))
  ;[1 1 1] Shoot at Rate of Fire
  (bind _output_get (Variables|Default|SetTime (+ DeltaSeconds (Variables|Default|GetTime))))
  (if (>= _output_get (Variables|Default|GetRateOfFire))
    (CallFunction|Shoot)
    (Variables|Default|SetTime 0.0)
    (Variables|Default|SetDirection (* -1 (Variables|Default|GetDirection)))
    (elif (Math|Float|NearlyEqual(Float) (Variables|Default|GetTime) (Variables|Default|GetRateOfFire) 0.5)
      (Transformation|SetActorLocation (Math|Vector|MakeVector (+ (.x _returnvalue) (* DeltaSeconds (* 500 (Variables|Default|GetDirection)))) (.y _returnvalue) (.z _returnvalue)) false false))))

(fn ConstructionScript)

(fn Shoot
  (bind _forward (CallFunction|GetForward))
  (bind _outactors (Actor|GetAllActorsOfClass "/Game/Runner_Content/Blueprints/BP_Player.BP_Player_C"))
  (bind _returnvalue (Game|SpawnActorfromClass "/Game/Runner_Content/Blueprints/BP_Bullet.BP_Bullet_C" (Math|Transform|MakeTransform (+ (.location (Transformation|GetActorTransform)) (* (Transformation|GetActorForwardVector) -2e+02)) (Math|Rotator|FindLookatRotation (Transformation|GetActorLocation) (Transformation|GetActorLocation (Utilities|Array|Get(acopy) _outactors))) "0.250000,0.250000,0.250000") "Undefined" 0 0))
  (Actor|SetLifeSpan _returnvalue 5.0))

(fn GetForward
  ;[1 1 1] Normalizes distance vector between enemy and player to create forward firing vector
  (bind _asbp_player (Utilities|Casting|CastToBP_Player (Game|GetPlayerCharacter 0)))
  (return (Math|Vector|Normalize (- (Transformation|GetActorLocation) (Transformation|GetActorLocation _asbp_player)))))