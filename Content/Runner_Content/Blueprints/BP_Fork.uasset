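; BP_Fork is a forked track tile in a runner game where the player turns left or right.
; Each turn box enables the player's CanTurn, flags the chosen side on BP_RunnerMode and moves its next spawn point to that side's attach point, resetting the secondary one.
; The left and right boxes have the game mode spawn a tunnel tile, then destroy the fork after a delay.
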(event OnComponentBeginOverlap(BoxLeft)
  (params (OverlappedComponent :type Primitive%20Component%20Object%20Reference) (OtherActor :type Actor%20Object%20Reference) (OtherComp :type Primitive%20Component%20Object%20Reference) (OtherBodyIndex :type Integer) (bFromSweep :type Boolean) (SweepResult :type Hit%20Result%20Structure%20%28by%20ref%29))
  (Utilities|Casting|CastToBP_Player OtherActor)
  (bind _asbp_runner_mode (Utilities|Casting|CastToBP_RunnerMode (Game|GetGameMode)))
  (Default|SpawnTunnelTile _asbp_runner_mode)
  (Utilities|FlowControl|Delay 1e+01)
  (Actor|DestroyActor))

(event OnComponentBeginOverlap(BoxRight)
  (params (OverlappedComponent :type Primitive%20Component%20Object%20Reference) (OtherActor :type Actor%20Object%20Reference) (OtherComp :type Primitive%20Component%20Object%20Reference) (OtherBodyIndex :type Integer) (bFromSweep :type Boolean) (SweepResult :type Hit%20Result%20Structure%20%28by%20ref%29))
  (Utilities|Casting|CastToBP_Player OtherActor)
  (bind _asbp_runner_mode (Utilities|Casting|CastToBP_RunnerMode (Game|GetGameMode)))
  (Default|SpawnTunnelTile _asbp_runner_mode)
  (Utilities|FlowControl|Delay 1e+01)
  (Actor|DestroyActor))

(event OnComponentBeginOverlap(BoxTurnLeft)
  (params (OverlappedComponent :type Primitive%20Component%20Object%20Reference) (OtherActor :type Actor%20Object%20Reference) (OtherComp :type Primitive%20Component%20Object%20Reference) (OtherBodyIndex :type Integer) (bFromSweep :type Boolean) (SweepResult :type Hit%20Result%20Structure%20%28by%20ref%29))
  ;[1 1 1] 'Fork' left
  (bind _asbp_player (Utilities|Casting|CastToBP_Player OtherActor))
  (Variables|/Game/Runner_Content/Blueprints/BP_Player.BP_Player_C|SetCanTurn _asbp_player true)
  (bind _output_get (Variables|Default|SetLeftTurn true))
  (bind _asbp_runner_mode (Utilities|Casting|CastToBP_RunnerMode (Game|GetGameMode)))
  (Variables|/Game/Runner_Content/Blueprints/BP_RunnerMode.BP_RunnerMode_C|SetLeft _asbp_runner_mode _output_get)
  (Variables|/Game/Runner_Content/Blueprints/BP_RunnerMode.BP_RunnerMode_C|SetRight _asbp_runner_mode false)
  (bind _attachtransform (CallFunction|GetAttachTransformLeft))
  (Variables|/Game/Runner_Content/Blueprints/BP_RunnerMode.BP_RunnerMode_C|SetNextSpawnPoint _asbp_runner_mode _attachtransform)
  (Variables|/Game/Runner_Content/Blueprints/BP_RunnerMode.BP_RunnerMode_C|SetNextSpawnPoint2 _asbp_runner_mode (Math|Transform|MakeTransform "0, 0, 0")))

(event OnComponentBeginOverlap(BoxTurnRight)
  (params (OverlappedComponent :type Primitive%20Component%20Object%20Reference) (OtherActor :type Actor%20Object%20Reference) (OtherComp :type Primitive%20Component%20Object%20Reference) (OtherBodyIndex :type Integer) (bFromSweep :type Boolean) (SweepResult :type Hit%20Result%20Structure%20%28by%20ref%29))
  ;[1 1 1] 'Fork' right
  (bind _asbp_player (Utilities|Casting|CastToBP_Player OtherActor))
  (Variables|/Game/Runner_Content/Blueprints/BP_Player.BP_Player_C|SetCanTurn _asbp_player true)
  (bind _output_get (Variables|Default|SetLeftTurn true))
  (bind _asbp_runner_mode (Utilities|Casting|CastToBP_RunnerMode (Game|GetGameMode)))
  (Variables|/Game/Runner_Content/Blueprints/BP_RunnerMode.BP_RunnerMode_C|SetRight _asbp_runner_mode _output_get)
  (Variables|/Game/Runner_Content/Blueprints/BP_RunnerMode.BP_RunnerMode_C|SetLeft _asbp_runner_mode false)
  (bind _attachtransform (CallFunction|GetAttachTransformRight))
  (Variables|/Game/Runner_Content/Blueprints/BP_RunnerMode.BP_RunnerMode_C|SetNextSpawnPoint _asbp_runner_mode _attachtransform)
  (Variables|/Game/Runner_Content/Blueprints/BP_RunnerMode.BP_RunnerMode_C|SetNextSpawnPoint2 _asbp_runner_mode (Math|Transform|MakeTransform "0, 0, 0")))

(event EventBeginPlay)

(event Collision|EventActorBeginOverlap
  (params (OtherActor :type Actor%20Object%20Reference)))

(event EventTick
  (params (DeltaSeconds :type Float%20%28single-precision%29)))

(fn ConstructionScript)

(fn GetAttachTransformLeft
  (return (Transformation|GetWorldTransform (Variables|Default|GetAttachPointLeft))))

(fn GetAttachTransformRight
  (return (Transformation|GetWorldTransform (Variables|Default|GetAttachPointRight))))