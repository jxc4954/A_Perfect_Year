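; Player character for a tunnel runner: flies forward automatically, shifts on input axes and makes gated 90-degree Q/E turns.
; Left mouse repeatedly fires cursor-aimed bullets ahead via a timer; right mouse launches a cooldown-limited light sonar.
; Tunnel hits or depleted health trigger explosion and lose screen; other hits cost health and check Score for a win.
; Enter after losing destroys the actor, whose Destroyed event respawns it at LastCheckpoint or a PlayerStart.
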(event OnComponentHit(CapsuleComponent)
  (params (HitComponent :type Primitive%20Component%20Object%20Reference) (OtherActor :type Actor%20Object%20Reference) (OtherComp :type Primitive%20Component%20Object%20Reference) (NormalImpulse :type Vector :default "0, 0, 0") (Hit :type Hit%20Result%20Structure%20%28by%20ref%29))
  ;[1 1 1] Self-Destruct on Hit
  (Utilities|Casting|CastToBP_Tunnel OtherActor
    (:then
      (Effects|SpawnEmitteratLocation "/Game/Particles/P_Explosion.P_Explosion" (Transformation|GetActorLocation) :!label _label)
      (Rendering|SetVisibility (Variables|Collision|GetCapsuleComponent) false true)
      (Variables|Movement|SetCanMove false)
      (Utilities|FlowControl|Delay 1.0)
      (bind _returnvalue (UserInterface|CreateWidget "/Game/Puzzle_Content/Widgets/W_LoseScreen.W_LoseScreen_C"))
      (UserInterface|Viewport|AddtoViewport _returnvalue 2)
      (Variables|Default|SetLose true))
    (:CastFailed
      (Utilities|Casting|CastToBP_Corner OtherActor
        (:then
          (goto _label))
        (:CastFailed
          (Utilities|Casting|CastToFbxScene_Fork4 OtherActor
            (:then
              (goto _label))
            (:CastFailed
              (Variables|Default|SetHealth (- (Variables|Default|GetHealth) 1e+01))
              (if (<= (Variables|Default|GetHealth) 0.0)
                (goto _label)
                (else
                  (if (>= (Variables|Default|GetHealth) 1e+02)
                    (Variables|Default|SetHealth 1e+02))
                  (if (>= (Variables|Default|GetScore) 1e+02)
                    (Variables|Movement|SetCanMove false)
                    (bind _returnvalue_2 (UserInterface|CreateWidget "/Game/Puzzle_Content/Widgets/W_WinScreen.W_WinScreen_C"))
                    (UserInterface|Viewport|AddtoViewport _returnvalue_2 2)))))))))))

(event EventBeginPlay
  ;[1 1 1] Spawn Player Camera
  (bind _returnvalue (UserInterface|CreateWidget "/Game/Runner_Content/Blueprints/Widgets/BP_Hud.BP_Hud_C"))
  (bind _output_get (Variables|Default|SetPlayerHud _returnvalue))
  (UserInterface|Viewport|AddtoViewport _output_get 0)
  (Variables|Movement|SetCanTurn false))

(event Collision|EventActorBeginOverlap
  (params (OtherActor :type Actor%20Object%20Reference)))

(event EventDestroyed
  ;[1 1 1] Respawn
  (CallFunction|SpawnPlayer (Variables|Default|GetLast%20Checkpoint) false))

(event EventTick
  (params (DeltaSeconds :type Float%20%28single-precision%29))
  ;[1 1 1] Move forward
  (if (Variables|Movement|GetCanMove)
    (Variables|/Script/Engine.MovementComponent|SetVelocity (Variables|Character|GetCharacterMovement) (* (Math|Vector|RotateVector (Variables|Movement|GetForwardSpeed) (Transformation|GetActorRotation)) DeltaSeconds))
    (else
      (Variables|/Script/Engine.MovementComponent|SetVelocity (Variables|Character|GetCharacterMovement) "0, 0, 0"))))

(event Input|AxisEvents|InputAxisVerticalMovement
  (params (AxisValue :type Float%20%28single-precision%29))
  (bind _capsulecomponent (Variables|Collision|GetCapsuleComponent))
  ;[1 1 1] Player Movement
  (if (Variables|Movement|GetCanMove)
    (Transformation|SetWorldLocation _capsulecomponent (+ (Transformation|GetWorldLocation _capsulecomponent) (* (* (Transformation|GetActorUpVector) (Variables|Movement|GetSpeed)) AxisValue)) false false)))

(event Input|AxisEvents|InputAxisHorizontalMovement
  (params (AxisValue :type Float%20%28single-precision%29))
  (bind _capsulecomponent (Variables|Collision|GetCapsuleComponent))
  ;[1 1 1] Player Movement
  (if (Variables|Movement|GetCanMove)
    (Transformation|SetWorldLocation _capsulecomponent (+ (Transformation|GetWorldLocation _capsulecomponent) (* (* (Transformation|GetActorRightVector) (Variables|Movement|GetSpeed)) AxisValue)) false false)))

(event Input|KeyboardEvents|E
  (params (Key :type Key%20Structure :default "AnyKey"))
  ;[1 1 1] Turn Right
  (:Pressed
    (if (Variables|Movement|GetCanTurn)
      (Transformation|SetActorRotation (Math|Rotator|CombineRotators (Transformation|GetActorRotation) "0,90.000000, 0"))
      (Variables|Movement|SetCanTurn false))))

(event Input|KeyboardEvents|Q
  (params (Key :type Key%20Structure :default "AnyKey"))
  ;[1 1 1] Turn Left
  (:Pressed
    (if (Variables|Movement|GetCanTurn)
      (Transformation|SetActorRotation (Math|Rotator|CombineRotators (Transformation|GetActorRotation) "0,-90.000000, 0"))
      (Variables|Movement|SetCanTurn false))))

(event Input|MouseEvents|LeftMouseButton
  (params (Key :type Key%20Structure :default "AnyKey"))
  ;[1 1 1] Fire Bullets
  (:Pressed
    (bind _returnvalue (Utilities|Time|SetTimerbyFunctionName 0 "Shoot" 0.25 true))
    (CallFunction|Shoot))
  (:Released
    (Utilities|Time|ClearandInvalidateTimerbyHandle _returnvalue)))

(event Input|KeyboardEvents|Enter
  (params (Key :type Key%20Structure :default "AnyKey"))
  ;[1 1 1] Open RPG
  (:Pressed
    (if (Variables|Default|GetLose)
      (Actor|DestroyActor)
      (Viewport|RemoveAllWidgets))))

(event Input|MouseEvents|RightMouseButton
  (params (Key :type Key%20Structure :default "AnyKey"))
  ;[1 1 1] Fire Light Sonar
  (:Pressed
    (if (Variables|Default|GetCanFireSonar)
      (CallFunction|Sonar)
      (Utilities|FlowControl|Delay 2.0)
      (Variables|Default|SetCanFireSonar true))))

(fn ConstructionScript)

(fn Seek
  (params (Target :type Vector))
  (bind _returnvalue (Transformation|GetActorLocation))
  (bind _returnvalue_2 (Transformation|GetActorRotation))
  (bind _maxspeed (Variables|Movement|GetMaxSpeed))
  (bind _returnvalue_3 (- Target _returnvalue))
  (bind _returnvalue_4 (Math|Vector|Normalize _returnvalue_3))
  (bind _returnvalue_5 (Math|Vector|UnrotateVector _returnvalue_4 _returnvalue_2))
  (bind _returnvalue_6 (* _returnvalue_5 _maxspeed))
  (if (Variables|Movement|GetCanMove)
    (Physics|AddImpulse (Variables|Character|GetCharacterMovement) (Math|Vector|RotateVector (Math|Vector|MakeVector 0.0 (.y _returnvalue_6) (.z _returnvalue_6)) (Transformation|GetActorRotation)) true)))

(fn Shoot
  (bind _returnvalue (Game|GetPlayerController 0))
  (bind _returnvalue_2 (Transformation|GetActorLocation))
  (bind _hitresult (Game|Player|GetHitResultUnderCursorbyChannel _returnvalue "TraceTypeQuery1" true))
  (bind _location (Collision|BreakHitResult _hitresult))
  (if (Variables|Movement|GetCanMove)
    ;[1 1 1] Checking if object is behind player
    (if (< (Math|Vector|DotProduct (Transformation|GetActorForwardVector) (Class|KismetMathLibrary|GetDirectionVector _location (Transformation|GetActorLocation))) 0.0)
      ;[1 1 1] Spawning Bullet
      (bind _returnvalue_3 (Game|SpawnActorfromClass "/Game/Runner_Content/Blueprints/BP_Bullet_IDK.BP_Bullet_IDK_C" (Math|Transform|MakeTransform (+ _returnvalue_2 (* (Transformation|GetActorForwardVector) 2e+02)) (Math|Rotator|FindLookatRotation _returnvalue_2 _location) "0.250000,0.250000,0.250000") "Undefined" 0 0))
      (Variables|Default|SetCanFire false)
      (Actor|SetLifeSpan _returnvalue_3 2.0))))

(fn Sonar
  (bind _returnvalue (Transformation|GetActorTransform))
  (bind _returnvalue_2 (Transformation|GetActorForwardVector))
  (bind _returnvalue_3 (* _returnvalue_2 2e+02))
  (bind _returnvalue_4 (+ (.location _returnvalue) _returnvalue_3))
  (bind _returnvalue_5 (Game|SpawnActorfromClass "/Game/Runner_Content/Blueprints/BP_LightSonar.BP_LightSonar_C" (Math|Transform|MakeTransform _returnvalue_4 (.rotation _returnvalue) "1.000000,1.000000,1.000000") "AlwaysSpawn" 0 0))
  (Variables|Default|SetCanFireSonar false)
  (Default|InitVelocity _returnvalue_5 _returnvalue_4 "1.000000, 0, 0" 1.75e+03)
  (Actor|SetLifeSpan _returnvalue_5 3.5))

(fn SpawnPlayer
  (params (Transform :type Transform) (Random :type Boolean))
  (if (Math|Vector|NotEqual(Vector) (.Location (Math|Transform|BreakTransform Transform)) "0, 0, 0" 0.0001)
    (bind _returnvalue (Game|SpawnActorfromClass "BP_Player_C" Transform "Undefined" 0 0))
    (bind _aspawn (Utilities|Casting|CastToPawn _returnvalue))
    (Variables|Default|SetPlayerPawn _aspawn)
    (else
      (bind _outactors (Actor|GetAllActorsOfClass "/Script/Engine.PlayerStart"))
      (if Random
        (bind _asplayer_start (Utilities|Casting|CastToPlayerStart (Utilities|Array|Get(acopy) _outactors (Math|Random|RandomInteger (Utilities|Array|Length _outactors)))))
        (Variables|Default|SetLast%20Spawn _asplayer_start)
        (else
          (bind _array_element (Utilities|Array|ForEachLoopwithBreak _outactors :!label _label)
            (:LoopBody
              (bind _asplayer_start_2 (Utilities|Casting|CastToPlayerStart _array_element))
              (Variables|Default|SetLast%20Spawn _asplayer_start_2)
              (goto _label Break))
            (:Completed
              _))))
      (bind _returnvalue_2 (Game|SpawnActorfromClass "BP_Player_C" (Transformation|GetActorTransform (Variables|Default|GetLast%20Spawn)) "Undefined" 0 0))
      (bind _aspawn_2 (Utilities|Casting|CastToPawn _returnvalue_2))
      (bind _output_get (Variables|Default|SetPlayerPawn _aspawn_2))))
  (Pawn|Possess (Game|GetPlayerController 0) _output_get))

(fn GetCheckpoint
  (bind _last_checkpoint (Variables|Default|GetLast%20Checkpoint))
  (return (Math|Vector|NotEqual(Vector) (.Location (Math|Transform|BreakTransform _last_checkpoint)) "0, 0, 0" 0.0001) _last_checkpoint))

(fn SetCheckpoint
  (params (Update :type Boolean))
  (if Update
    (bind _output_get (Variables|Default|SetLast%20Checkpoint (Transformation|GetActorTransform)))
    (else
      (Variables|Default|SetLast%20Checkpoint "")))
  (return (Math|Vector|NotEqual(Vector) (.Location (Math|Transform|BreakTransform _output_get)) "0, 0, 0" 0.0001)))