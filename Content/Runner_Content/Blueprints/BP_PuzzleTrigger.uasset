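; BP_PuzzleTrigger is an overlap trigger in the runner game that pauses the player to present a puzzle.
; When BP_Player enters, it spawns the Puzzle class ahead of the player, passing it the runner camera, a player-based rotation and a scale.
; It disables player movement and gravity and enables click events.
; It then spawns a BP_PuzzleCamera forward of PlayerCam and blends the view to it.
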(event Collision|EventActorBeginOverlap
  (params (OtherActor :type Actor%20Object%20Reference))
  (bind _returnvalue (Transformation|GetActorTransform))
  (bind _playercam (Variables|Default|GetplayerCam))
  (bind _returnvalue_2 (Transformation|GetActorTransform _playercam))
  (bind (_location _rotation _scale) (Math|Transform|BreakTransform _returnvalue))
  (bind (_location_2 _rotation_2 _scale_2) (Math|Transform|BreakTransform _returnvalue_2))
  ;[1 1 1] Spawning a puzzle
  (bind _asbp_player (Utilities|Casting|CastToBP_Player OtherActor))
  (bind _outactors (Actor|GetAllActorsOfClass "/Game/Runner_Content/Blueprints/BP_RunnerCamera.BP_RunnerCamera_C"))
  (Game|SpawnActorfromClass (Variables|Default|Getpuzzle) (Math|Transform|MakeTransform (+ _location (* (Transformation|GetActorForwardVector _asbp_player) 2e+02)) _rotation _scale) "Undefined" 0 (Utilities|Array|Get(acopy) _outactors) (Math|Rotator|MakeRotator (.Roll (Math|Rotator|BreakRotator (Transformation|GetActorRotation _asbp_player))) (+ (.Pitch (Math|Rotator|BreakRotator (Transformation|GetActorRotation _asbp_player))) 9e+01) (.Yaw (Math|Rotator|BreakRotator (Transformation|GetActorRotation _asbp_player)))) (Variables|Default|GetpuzzleScale))
  ;[1 1 1] Keeping player in place
  (Variables|/Game/Runner_Content/Blueprints/BP_Player.BP_Player_C|SetCanMove _asbp_player false)
  (Variables|/Script/Engine.PlayerController|SetbEnableClickEvents (Game|GetPlayerController 0) true)
  (bind _outactors_2 (Actor|GetAllActorsOfClass "/Game/Runner_Content/Blueprints/BP_Player.BP_Player_C"))
  (Variables|/Script/Engine.CharacterMovementComponent|SetGravityScale (Variables|/Script/Engine.Character|GetCharacterMovement (Utilities|Array|Get(acopy) _outactors_2)) 0.0)
  ;[1 1 1] Moving to a different camera to view the puzzle
  (bind _returnvalue_3 (Game|SpawnActorfromClass "/Game/Puzzle_Content/Blueprints/BP_PuzzleCamera.BP_PuzzleCamera_C" (Math|Transform|MakeTransform (+ (* (Transformation|GetActorForwardVector _playercam) 7e+02) _location_2) _rotation_2 _scale_2) "Undefined" 0 0))
  (Game|Player|SetViewTargetwithBlend (Game|GetPlayerController 0) _returnvalue_3 0.3 "VTBlend_Linear" 0.0 false))

(fn ConstructionScript)