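; Runner camera actor that becomes player 0's view target on BeginPlay and trails the player character.
; Each Tick it rebuilds its position from the relative offset to the character, pinning X to TrailDistance, keeping Y and Z, and rotating by the character's rotation.
; The Turn function re-places that offset around the character using a supplied rotation, then snaps the camera to that rotation, which Tick never changes.
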(event EventBeginPlay
  (Game|Player|SetViewTargetwithBlend (Game|GetPlayerController 0) self 0.0 "VTBlend_Linear" 0.0 false))

(event Collision|EventActorBeginOverlap
  (params (OtherActor :type Actor%20Object%20Reference)))

(event EventTick
  (params (DeltaSeconds :type Float%20%28single-precision%29))
  (bind _returnvalue (Game|GetPlayerCharacter 0))
  (bind _returnvalue_2 (Transformation|GetActorTransform))
  (bind _traildistance (Variables|Default|GetTrailDistance))
  (bind _returnvalue_3 (Transformation|GetActorTransform _returnvalue))
  (bind _returnvalue_4 (Class|KismetMathLibrary|ConvertTransformtoRelative _returnvalue_2 _returnvalue_3))
  (bind (_x _y _z) (Math|Vector|BreakVector (.location _returnvalue_4)))
  (Transformation|SetActorLocation (- (Transformation|GetActorLocation _returnvalue) (Math|Vector|RotateVector (Math|Vector|MakeVector (Math|Float|Clamp(Float) _x _traildistance _traildistance) _y _z) (Transformation|GetActorRotation _returnvalue))) false false))

(fn ConstructionScript)

(fn Turn
  (params (Rotation :type Rotator))
  (bind _returnvalue (Game|GetPlayerCharacter 0))
  (Transformation|SetActorLocation (- (Transformation|GetActorLocation _returnvalue) (Math|Vector|RotateVector (.location (Class|KismetMathLibrary|ConvertTransformtoRelative (Transformation|GetActorTransform) (Transformation|GetActorTransform _returnvalue))) Rotation)) false false)
  (Transformation|SetActorRotation Rotation))