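; Runner game mode that procedurally builds the tunnel course at BeginPlay by repeatedly calling SpawnTunnelTile.
; Each tile's attach transform becomes the next spawn point, with a corner or fork replacing a straight when TileCount hits a multiple of seven.
; Forks set a second spawn point, after which straight tunnels extend both branches.
; Mouse-seek steering, left/right branch selection and puzzle-trigger spawning are unconnected, so Tick only performs casts.
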(event EventBeginPlay
  ;[1 1 1] Create Tiles
  (for _index (range 0 20)
    (CallFunction|SpawnTunnelTile)
    (Math|Float|IncrementFloat (Variables|Default|GetTileCount))))

(event EventTick
  (params (DeltaSeconds :type Float%20%28single-precision%29))
  ;[1 1 1] Player Mouse Tracking
  (bind _asbp_runner_controller (Utilities|Casting|CastToBP_RunnerController (Game|GetPlayerController 0)))
  (bind _asbp_player (Utilities|Casting|CastToBP_Player (Game|Player|GetPlayerPawn 0))))

(fn ConstructionScript)

(fn SpawnTunnelTile
  (bind _tilecount (Variables|Default|GetTileCount))
  ;[1 1 1] Check tile spawn count
  (if (and (== (Math|Float|%(Float) _tilecount 7.0) 0.0) (!= _tilecount 0.0)) ; Every 7 spawns 'Turn'
    (if (== (Math|Float|%(Float) _tilecount 3.0) 0.0)
      ;[1 1 1] Spawn 'Turn' segment
      (bind _returnvalue (Game|SpawnActorfromClass "/Game/Runner_Content/Blueprints/BP_Fork.BP_Fork_C" (Variables|Default|GetNextSpawnPoint) "Undefined" 0 0))
      (bind _asbp_fork (Utilities|Casting|CastToBP_Fork _returnvalue))
      (bind _attachtransform (Default|GetAttachTransformLeft _asbp_fork))
      (Variables|Default|SetNextSpawnPoint _attachtransform)
      (bind _attachtransform_2 (Default|GetAttachTransformRight _asbp_fork))
      (Variables|Default|SetNextSpawnPoint2 _attachtransform_2)
      (Math|Float|IncrementFloat (Variables|Default|GetTileCount))
      (else
        (bind _returnvalue_2 (Game|SpawnActorfromClass "/Game/Runner_Content/Blueprints/BP_Corner.BP_Corner_C" (Variables|Default|GetNextSpawnPoint) "Undefined" 0 0))
        (bind _asbp_corner (Utilities|Casting|CastToBP_Corner _returnvalue_2))
        (bind _attachtransform_3 (Default|GetAttachTransform _asbp_corner))
        (Variables|Default|SetNextSpawnPoint _attachtransform_3)
        (Math|Float|IncrementFloat (Variables|Default|GetTileCount))))
    (else
      ;[1 1 1] Spawn 'Tunnel' segments
      (if (== (Variables|Default|GetNextSpawnPoint2) (Math|Transform|MakeTransform "0, 0, 0")) ; If 'Forking' spawn down both paths
        (bind _returnvalue_3 (Game|SpawnActorfromClass "/Game/Runner_Content/Blueprints/BP_Tunnel.BP_Tunnel_C" (Variables|Default|GetNextSpawnPoint) "Undefined" 0 0))
        (bind _asbp_tunnel (Utilities|Casting|CastToBP_Tunnel _returnvalue_3))
        (bind _attachtransform_4 (Default|GetAttachTransform _asbp_tunnel))
        (Variables|Default|SetNextSpawnPoint _attachtransform_4)
        (Math|Float|IncrementFloat (Variables|Default|GetTileCount))
        (else
          (bind _returnvalue_4 (Game|SpawnActorfromClass "/Game/Runner_Content/Blueprints/BP_Tunnel.BP_Tunnel_C" (Variables|Default|GetNextSpawnPoint) "Undefined" 0 0))
          (bind _asbp_tunnel_2 (Utilities|Casting|CastToBP_Tunnel _returnvalue_4))
          (bind _attachtransform_5 (Default|GetAttachTransform _asbp_tunnel_2))
          (Variables|Default|SetNextSpawnPoint _attachtransform_5)
          (Math|Float|IncrementFloat (Variables|Default|GetTileCount)
            (:%20%20
              (bind _returnvalue_5 (Game|SpawnActorfromClass "/Game/Runner_Content/Blueprints/BP_Tunnel.BP_Tunnel_C" (Variables|Default|GetNextSpawnPoint2) "Undefined" 0 0))
              (bind _asbp_tunnel_3 (Utilities|Casting|CastToBP_Tunnel _returnvalue_5))
              (bind _attachtransform_6 (Default|GetAttachTransform _asbp_tunnel_3))
              (Variables|Default|SetNextSpawnPoint2 _attachtransform_6)
              (Math|Float|IncrementFloat (Variables|Default|GetTileCount)))))))))