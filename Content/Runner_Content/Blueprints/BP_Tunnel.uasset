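; BP_Tunnel is a tunnel tile for an endless runner that populates itself and keeps the track extending.
; On BeginPlay it randomly spawns either a BP_Enemy or a BP_Obstacle at a random point around its AttachPoint, using the Box extent as bounds.
; When BP_Player overlaps the Box, it asks BP_RunnerMode to spawn the next tile, then destroys itself after a delay.
; GetAttachTransform exposes the AttachPoint's world transform.
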(event OnComponentBeginOverlap(Box)
  (params (OverlappedComponent :type Primitive%20Component%20Object%20Reference) (OtherActor :type Actor%20Object%20Reference) (OtherComp :type Primitive%20Component%20Object%20Reference) (OtherBodyIndex :type Integer) (bFromSweep :type Boolean) (SweepResult :type Hit%20Result%20Structure%20%28by%20ref%29))
  ;[1 1 1] Spawn Next Tile and Self-Destruct
  (Utilities|Casting|CastToBP_Player OtherActor)
  (bind _asbp_runner_mode (Utilities|Casting|CastToBP_RunnerMode (Game|GetGameMode)))
  (Default|SpawnTunnelTile _asbp_runner_mode)
  (Utilities|FlowControl|Delay 1e+01)
  (Actor|DestroyActor))

(event EventBeginPlay
  (bind _box (Variables|Default|GetBox))
  (bind _attachpoint (Variables|Default|GetAttachPoint))
  (bind _returnvalue (Transformation|GetWorldLocation _attachpoint))
  (bind _boxextent (Variables|/Script/Engine.BoxComponent|GetBoxExtent _box))
  (bind _returnvalue_2 (Math|Random|RandomPointinBoundingBox _returnvalue _boxextent))
  ;[1 1 1] Spawn Enemies or Obstacles
  (bind _attachtransform (CallFunction|GetAttachTransform))
  (switch int (Math|Random|RandomIntegerinRange 0 1)
    (:Default
      (Game|SpawnActorfromClass "/Game/Runner_Content/Blueprints/BP_Enemy.BP_Enemy_C" (Math|Transform|MakeTransform _returnvalue_2 (.rotation _attachtransform) "1,1,1") "AlwaysSpawn" 0 0 :!label _label))
    (:0
      (goto _label))
    (:1
      (Game|SpawnActorfromClass "/Game/Runner_Content/Blueprints/BP_Obstacle.BP_Obstacle_C" (Math|Transform|MakeTransform _returnvalue_2 "0.000000, 0, 0" "1,1,1") "AlwaysSpawn" 0 0))))

(event Collision|EventActorBeginOverlap
  (params (OtherActor :type Actor%20Object%20Reference)))

(event EventTick
  (params (DeltaSeconds :type Float%20%28single-precision%29)))

(fn ConstructionScript)

(fn GetAttachTransform
  ;[1 1 1] Get tile transform
  (return (Transformation|GetWorldTransform (Variables|Default|GetAttachPoint))))